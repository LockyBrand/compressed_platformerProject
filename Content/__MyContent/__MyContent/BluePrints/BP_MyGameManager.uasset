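; Game manager Blueprint that owns the game state: running, won, lost or abandon.
; Init has the game mode create the UI, initializes the player, caches destructible floor and coin locations, and sets Running from inside those nested loops.
; SetState switches widgets, mouse cursor and pause on each state change.
; ResetGame returns the player to the first PlayerStart, reinitializes them and spawns new floors where existing ones are broken.
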(event `self.ReceiveBeginPlay`)

(fn `GetState`
  (returns (State :type "/Game/__MyContent/BluePrints/E_MyGameStates Enum"))
  (return (`self.Current Game State`)))

(fn `Init`
  (bind _asbp_my_game_mode (cast `/Game/__MyContent/BluePrints/BP_MyGameMode` (`GameplayStatics.GetGameMode`)))
  (`/Game/__MyContent/BluePrints/BP_MyGameMode.create UI` _asbp_my_game_mode)
  (`/Game/ThirdPersonBP/Blueprints/ThirdPersonCharacter.Init` (`self.MyPlayer`))
  (bind _outactors (`GameplayStatics.GetAllActorsOfClass` "/Game/__MyContent/BluePrints/BP_destructableFloor.BP_destructableFloor_C"))
  (for (_array_element _array_index) _outactors
    (`KismetArrayLibrary.Array_Insert` (`self.destructable floor locations`) (`self.K2_GetActorLocation` _array_element) _array_index)
    (bind _outactors_2 (`GameplayStatics.GetAllActorsOfClass` "/Game/__MyContent/BluePrints/BP_coin.BP_coin_C"))
    (for (_array_element_2 _array_index_2) _outactors_2
      (`KismetArrayLibrary.Array_Insert` (`self.coin locations`) (`self.K2_GetActorLocation` _array_element_2) _array_index_2)
      (`self.SetState` "NewEnumerator0"))))

(fn `resetGame`
  (bind _outactors (`GameplayStatics.GetAllActorsOfClass` "/Script/Engine.PlayerStart"))
  (`self.K2_SetActorLocation` (`self.MyPlayer`) (`self.K2_GetActorLocation` (`|GetArrayItem` _outactors)) false false)
  (`/Game/ThirdPersonBP/Blueprints/ThirdPersonCharacter.Init` (`self.MyPlayer`))
  (bind _outactors_2 (`GameplayStatics.GetAllActorsOfClass` "/Game/__MyContent/BluePrints/BP_destructableFloor.BP_destructableFloor_C"))
  (for _array_element _outactors_2
    (if (`/Game/__MyContent/BluePrints/BP_destructableFloor.is broken?` _array_element)
      (`|SpawnActorFromClass` "/Game/__MyContent/BluePrints/BP_destructableFloor.BP_destructableFloor_C" (`KismetMathLibrary.Conv_VectorToTransform` (`self.K2_GetActorLocation` _array_element)) "Undefined" "OverrideRootScale" null null))))

(fn `SetState`
  (params (`New State` :type "/Game/__MyContent/BluePrints/E_MyGameStates Enum" :default "NewEnumerator0"))
  (if (`|EnumInequality` `New State` (`self.Current Game State`))
    (`/Game/__MyContent/BluePrints/BP_MyFunctionLibrary.Hide UI`)
    (bind _output_get (set `self.Current Game State` `New State`))
    (switch `/Game/__MyContent/BluePrints/E_MyGameStates` _output_get
      (:`NewEnumerator0`
        (`/Game/__MyContent/BluePrints/BP_MyFunctionLibrary.Show Mouse` false)
        (`GameplayStatics.SetGamePaused` false)
        (`self.show HUD` true))
      (:`NewEnumerator1`
        (`Widget.SetVisibility` (`self.widget_WIN`) "Visible")
        (`/Game/__MyContent/BluePrints/BP_MyFunctionLibrary.Show Mouse` true :!label _label)
        (`GameplayStatics.SetGamePaused` true))
      (:`NewEnumerator2`
        (`Widget.SetVisibility` (`self.widget_LOSE`) "Visible")
        (goto _label))
      (:`NewEnumerator3`
        (`Widget.SetVisibility` (`self.widget_abandon`) "Visible")
        (goto _label)))))

(fn `show HUD`
  (params (`visible?` :type Boolean))
  (if `visible?`
    (`Widget.SetVisibility` (`self.widget_HealthBar`) "Visible")
    (`Widget.SetVisibility` (`self.widget_keys`) "Visible")
    (else
      (`Widget.SetVisibility` (`self.widget_HealthBar`) "Visible"))))

(fn `UserConstructionScript`)