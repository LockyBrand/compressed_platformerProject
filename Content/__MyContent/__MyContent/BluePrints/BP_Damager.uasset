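; BP_Damager is a damage volume that drains health from a player-tagged ThirdPersonCharacter while it stays inside.
; Collision overlap events store the player and toggle an inside flag, with StartDamage resetting the accumulated damage to zero on each entry.
; While inside, Tick calls ContinueDamage, which applies frame-rate-independent damage through ChangeHealth until the running total reaches the per-visit maximum.
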(event `self.ReceiveTick`
  (params (DeltaSeconds :type "Float (single-precision)"))
  (if (`self.inside volume`)
    (`self.continue damage`)))

(event `self.colision volume.OnComponentBeginOverlap`
  (params (OverlappedComponent :type "PrimitiveComponent Object Reference") (OtherActor :type "Actor Object Reference") (OtherComp :type "PrimitiveComponent Object Reference") (OtherBodyIndex :type Integer) (bFromSweep :type Boolean) (SweepResult :type "HitResult Structure (by ref)"))
  (if (`self.ActorHasTag` OtherActor "Tag_Player")
    (bind _asthird_person_character (cast `/Game/ThirdPersonBP/Blueprints/ThirdPersonCharacter` OtherActor))
    (set `self.inside volume` true)
    (set `self.player` _asthird_person_character)
    (`self.start damage`)))

(event `self.colision volume.OnComponentEndOverlap`
  (params (OverlappedComponent :type "PrimitiveComponent Object Reference") (OtherActor :type "Actor Object Reference") (OtherComp :type "PrimitiveComponent Object Reference") (OtherBodyIndex :type Integer))
  (if (`self.ActorHasTag` OtherActor "Tag_Player")
    (cast `/Game/ThirdPersonBP/Blueprints/ThirdPersonCharacter` OtherActor)
    (set `self.inside volume` false)))

(fn `continue damage`
  (bind _returnvalue (* (`self.damage rate`) (`GameplayStatics.GetWorldDeltaSeconds`)))
  (if (< (`self.accum damage`) (`self.MAX damge`))
    (set `self.accum damage` (+ _returnvalue (`self.accum damage`))) ; increase accumulated damge by damge rate
    (`/Game/ThirdPersonBP/Blueprints/ThirdPersonCharacter.change Health` (`self.player`) (* _returnvalue -1.0))))

(fn `start damage`
  (bind _output_get (set `self.accum damage` 0.0))
  (if (> _output_get (`self.MAX damge`))
    (set `self.accum damage` (`self.MAX damge`)))
  (`/Game/ThirdPersonBP/Blueprints/ThirdPersonCharacter.change Health` (`self.player`) (* (`self.accum damage`) -1.0)))

(fn `UserConstructionScript`)