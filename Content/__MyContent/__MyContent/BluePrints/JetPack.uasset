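; Jetpack pickup that spins in place and grants the player a jetpack on touch.
; A capsule overlap checks the actor against MyPlayer from the Game Manager, sets HasJetpack and adds an upward force to the character's movement.
; It then plays a power-up sound and hides itself for a few seconds before reappearing, without changing its collision.
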(event `self.ReceiveTick`
  (params (DeltaSeconds :type "Float (single-precision)"))
  (`SceneComponent.K2_AddLocalRotation` (`self.DefaultSceneRoot`) (struct :`Yaw` 1.0) false false))

(event `self.Capsule.OnComponentBeginOverlap`
  (params (OverlappedComponent :type "PrimitiveComponent Object Reference") (OtherActor :type "Actor Object Reference") (OtherComp :type "PrimitiveComponent Object Reference") (OtherBodyIndex :type Integer) (bFromSweep :type Boolean) (SweepResult :type "HitResult Structure (by ref)"))
  (bind _mygamemanager (`/Game/__MyContent/BluePrints/BP_MyFunctionLibrary.get game manager`))
  (bind _myplayer (`/Game/__MyContent/BluePrints/BP_MyGameManager.MyPlayer` _mygamemanager))
  (if (== _myplayer OtherActor)
    (set `/Game/ThirdPersonBP/Blueprints/ThirdPersonCharacter.has jetpack` true _myplayer)
    (`CharacterMovementComponent.AddForce` (`Character.CharacterMovement` _myplayer) (0.0 0.0 1000.0))
    (`GameplayStatics.PlaySoundAtLocation` "/Game/__MyContent/audio/SC_PowerUp.SC_PowerUp" (`self.K2_GetActorLocation`) (struct) 1.0 1.0 0.0 null null null)
    (`self.SetActorHiddenInGame` true)
    (`KismetSystemLibrary.Delay` 5.0)
    (`self.SetActorHiddenInGame` false)))

(fn `UserConstructionScript`)