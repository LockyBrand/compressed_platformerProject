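; BP_simpleDoor is a sliding door actor that closes when the game manager's player overlaps its box trigger.
; Each overlap restarts the CloseDoor timeline, whose float track blends toward a DistanceToClosePos offset along Y.
; The lerp re-reads the current world location every update, so movement accumulates, and writes it as relative location.
; The construction script assigns the configurable Mesh to the static mesh component.
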(event `self.Box.OnComponentBeginOverlap`
  (params (OverlappedComponent :type "PrimitiveComponent Object Reference") (OtherActor :type "Actor Object Reference") (OtherComp :type "PrimitiveComponent Object Reference") (OtherBodyIndex :type Integer) (bFromSweep :type Boolean) (SweepResult :type "HitResult Structure (by ref)"))
  (bind _returnvalue (`self.K2_GetActorLocation`))
  (bind _mygamemanager (`/Game/__MyContent/BluePrints/BP_MyFunctionLibrary.get game manager`))
  (if (== (`/Game/__MyContent/BluePrints/BP_MyGameManager.MyPlayer` _mygamemanager) OtherActor)
    (bind (_direction _move_float) (`Timeline|close door` :!via `PlayFromStart`)
      (:`Update`
        (`self.K2_SetActorRelativeLocation` (`KismetMathLibrary.VLerp` _returnvalue (`KismetMathLibrary.MakeVector` (.x _returnvalue) (+ (.y _returnvalue) (`self.distanceToClosePos`)) (.z _returnvalue)) _move_float))))))

(fn `UserConstructionScript`
  (`StaticMeshComponent.SetStaticMesh` (`self.StaticMesh`) (`self.Mesh`)))