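; Cube enemy that deals heavy damage when the player touches its hit boxes and has a destructible weak point.
; Player overlap on the weak point fractures the cube with radial damage, spawns a key at its start location, then hides the debris after a delay.
; Timeline logic for lunging between player and rally point, then rotating toward the target, is present but has no trigger in the graph.
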(event `self.ReceiveBeginPlay`
  ;[1 1 1] cube movement and points to run to and from
  (`KismetSystemLibrary.Delay` 0.5)
  (bind _mygamemanager (`/Game/__MyContent/BluePrints/BP_MyFunctionLibrary.get game manager`))
  (set `self.rally point` (`self.K2_GetActorLocation`))
  (set `self.player` (`/Game/__MyContent/BluePrints/BP_MyGameManager.MyPlayer` _mygamemanager))
  (set `self.escape position` (`self.K2_GetActorLocation` (`self.player`))))

(event `self.hitBoxes.OnComponentBeginOverlap`
  (params (OverlappedComponent :type "PrimitiveComponent Object Reference") (OtherActor :type "Actor Object Reference") (OtherComp :type "PrimitiveComponent Object Reference") (OtherBodyIndex :type Integer) (bFromSweep :type Boolean) (SweepResult :type "HitResult Structure (by ref)"))
  ;[1 1 1] collision and damager
  (if (not (`self.cube destroyed`))
    (bind _mygamemanager (`/Game/__MyContent/BluePrints/BP_MyFunctionLibrary.get game manager`))
    (bind _myplayer (`/Game/__MyContent/BluePrints/BP_MyGameManager.MyPlayer` _mygamemanager))
    (if (== OtherActor _myplayer)
      (`/Game/ThirdPersonBP/Blueprints/ThirdPersonCharacter.change Health` _myplayer -50.0))))

(event `self.weak point.OnComponentBeginOverlap`
  (params (OverlappedComponent :type "PrimitiveComponent Object Reference") (OtherActor :type "Actor Object Reference") (OtherComp :type "PrimitiveComponent Object Reference") (OtherBodyIndex :type Integer) (bFromSweep :type Boolean) (SweepResult :type "HitResult Structure (by ref)"))
  (bind _cube_dm (`self.Cube_DM`))
  ;[1 1 1] collision and damager
  (bind _mygamemanager (`/Game/__MyContent/BluePrints/BP_MyFunctionLibrary.get game manager`))
  (if (== OtherActor (`/Game/__MyContent/BluePrints/BP_MyGameManager.MyPlayer` _mygamemanager))
    (`DestructibleComponent.ApplyRadiusDamage` _cube_dm 20.0 (`SceneComponent.K2_GetComponentLocation` _cube_dm) 20.0 0.0 false)
    (`self.spawn key` (`self.cube destroyed`))
    (`KismetSystemLibrary.Delay` 5.0)
    (`self.hide cube debis`)))

(fn `hide cube debis`
  (set `self.cube destroyed` true)
  (`SceneComponent.SetVisibility` (`self.Sphere`) false false)
  (`SceneComponent.SetVisibility` (`self.Sphere1`) false false)
  (`SceneComponent.SetVisibility` (`self.weak point`) false false)
  (`SceneComponent.SetVisibility` (`self.hitBoxes`) false false)
  (`SceneComponent.SetVisibility` (`self.Cube_DM`) false false)
  (`self.SetActorEnableCollision` false))

(fn `spawn key`
  (params (`is cube destroyed` :type Boolean))
  (if (not `is cube destroyed`)
    (`GameplayStatics.PlaySoundAtLocation` "/Game/__MyContent/audio/SC_explosion.SC_explosion" (`self.K2_GetActorLocation`) (struct) 1.0 1.0 0.0 null null null)
    (bind _returnvalue (`|SpawnActorFromClass` "/Game/__MyContent/BluePrints/key_BP.key_BP_C" (`KismetMathLibrary.Conv_VectorToTransform` (`self.rally point`)) "Undefined" "OverrideRootScale" null null))
    (`self.SetActorHiddenInGame` _returnvalue false)
    (`PrimitiveComponent.SetCollisionEnabled` (`/Game/__MyContent/BluePrints/key_BP.Capsule` _returnvalue) "QueryAndPhysics")
    (`SceneComponent.SetVisibility` (`self.Sphere1`) false false)
    (`SceneComponent.SetVisibility` (`self.Sphere`) false false)
    (set `self.cube destroyed` true)))

(fn `UserConstructionScript`
  (`PrimitiveComponent.SetMaterial` (`self.Cube_DM`) 0 (`self.material`)))