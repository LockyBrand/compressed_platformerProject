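; Blueprint function library of shared helpers for cursor, game manager and UI control.
; ShowMouse sets the first player's cursor visibility and switches input mode to UI-only or game-only to match.
; GetGameManager casts the game mode to BP_MyGameMode and returns its Manager reference.
; HideUI finds every top-level UserWidget and sets it hidden.
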(fn `get game manager`
  (returns (MyGameManager :type "/Game/__MyContent/BluePrints/BP_MyGameManager Object Reference"))
  (bind _asbp_my_game_mode (cast `/Game/__MyContent/BluePrints/BP_MyGameMode` (`GameplayStatics.GetGameMode` null)))
  (return (`/Game/__MyContent/BluePrints/BP_MyGameMode.manager` _asbp_my_game_mode)))

(fn `Hide UI`
  (bind _foundwidgets (`WidgetBlueprintLibrary.GetAllWidgetsOfClass` null "/Script/UMG.UserWidget"))
  (for _array_element _foundwidgets
    (`Widget.SetVisibility` _array_element "Hidden")))

(fn `Show Mouse`
  (params (visible :type Boolean))
  (bind _returnvalue (`GameplayStatics.GetPlayerController` null))
  (bind _output_get (set `PlayerController.bShowMouseCursor` visible _returnvalue))
  (if _output_get
    (`WidgetBlueprintLibrary.SetInputMode_UIOnlyEx` _returnvalue null)
    (else
      (`WidgetBlueprintLibrary.SetInputMode_GameOnly` _returnvalue))))