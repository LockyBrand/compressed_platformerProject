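; Key pickup actor that spins constantly and starts hidden with collision disabled; nothing here reveals it.
; On capsule overlap with the game manager's player, it plays a key sound unless SoundPlayed is set, then hides and disables collision again.
; It increments the key widget's count and briefly shows the got-keys widget.
; SoundPlayed is never set in this Blueprint.
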(event `self.ReceiveBeginPlay`
  (`self.SetActorHiddenInGame` true)
  (`PrimitiveComponent.SetCollisionEnabled` (`self.Capsule`) "NoCollision")
  (`PrimitiveComponent.SetCollisionEnabled` (`self.Cube2`) "NoCollision")
  (`PrimitiveComponent.SetCollisionEnabled` (`self.eer`) "NoCollision")
  (`PrimitiveComponent.SetCollisionEnabled` (`self.Cube`) "NoCollision")
  (`PrimitiveComponent.SetCollisionEnabled` (`self.Cube1`) "NoCollision"))

(event `self.ReceiveTick`
  (params (DeltaSeconds :type "Float (single-precision)"))
  (`SceneComponent.K2_AddLocalRotation` (`self.Capsule`) (struct :`Yaw` 1.0) false false))

(event `self.Capsule.OnComponentBeginOverlap`
  (params (OverlappedComponent :type "PrimitiveComponent Object Reference") (OtherActor :type "Actor Object Reference") (OtherComp :type "PrimitiveComponent Object Reference") (OtherBodyIndex :type Integer) (bFromSweep :type Boolean) (SweepResult :type "HitResult Structure (by ref)"))
  (bind _mygamemanager (`/Game/__MyContent/BluePrints/BP_MyFunctionLibrary.get game manager`))
  (if (== OtherActor (`/Game/__MyContent/BluePrints/BP_MyGameManager.MyPlayer` _mygamemanager))
    (if (not (`self.sound played`))
      (`GameplayStatics.PlaySoundAtLocation` "/Game/__MyContent/audio/SC_keyNoise.SC_keyNoise" (`self.K2_GetActorLocation`) (struct) 1.0 1.0 0.0 null null null))
    (`self.SetActorHiddenInGame` true)
    (`PrimitiveComponent.SetCollisionEnabled` (`self.Capsule`) "NoCollision")
    (`PrimitiveComponent.SetCollisionEnabled` (`self.Cube`) "NoCollision")
    (`PrimitiveComponent.SetCollisionEnabled` (`self.eer`) "NoCollision")
    (`PrimitiveComponent.SetCollisionEnabled` (`self.Cube1`) "NoCollision")
    (`PrimitiveComponent.SetCollisionEnabled` (`self.Cube2`) "NoCollision")
    (bind _mygamemanager_2 (`/Game/__MyContent/BluePrints/BP_MyFunctionLibrary.get game manager`))
    (bind _widget_gotkeys (`/Game/__MyContent/BluePrints/BP_MyGameManager.widget_gotKeys` _mygamemanager_2))
    (`Widget.SetVisibility` _widget_gotkeys "Visible")
    (bind _widget_keys (`/Game/__MyContent/BluePrints/BP_MyGameManager.widget_keys` _mygamemanager_2))
    (bind _result (`/Engine/EditorBlueprintResources/StandardMacros.IncrementInt` (`/Game/__MyContent/widgets/widget_keys.key amount` _widget_keys))
      (:`  `
        (set `/Game/__MyContent/widgets/widget_keys.key amount` _result _widget_keys)
        (`KismetSystemLibrary.Delay` 1.0)
        (`Widget.SetVisibility` _widget_gotkeys "Hidden")))))

(fn `UserConstructionScript`)