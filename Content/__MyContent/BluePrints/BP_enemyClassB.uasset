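; BP_enemyClassB is an enemy actor that patrols waypoints and deals damage over time to the player.
; Box overlap starts a damage timeline that drains health to zero, stopping two seconds after the player leaves.
; BeginPlay caches the player from the game manager and starts a movement timeline meant to lerp between three waypoints.
; That timeline's handlers advance the waypoint indices, optionally reverse at path end, and trigger a look-at rotation timeline.
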(event `self.Box.OnComponentBeginOverlap`
  (params (OverlappedComponent :type "PrimitiveComponent Object Reference") (OtherActor :type "Actor Object Reference") (OtherComp :type "PrimitiveComponent Object Reference") (OtherBodyIndex :type Integer) (bFromSweep :type Boolean) (SweepResult :type "HitResult Structure (by ref)"))
  (bind _player (`self.player`))
  ;[1 1 1] damage over time
  (if (== OtherActor _player)
    (bind (_direction _damage) (`Timeline|damage over time` :!via `PlayFromStart`)
      (:`Update`
        (bind _health_points (`/Game/ThirdPersonBP/Blueprints/ThirdPersonCharacter.getHealth` _player))
        (bind _returnvalue (* _damage -1.0))
        (if (> _returnvalue (* _health_points -1.0))
          (`/Game/ThirdPersonBP/Blueprints/ThirdPersonCharacter.change Health` _player _returnvalue)
          (else
            (`TimelineComponent.Stop` (`self.damage over time`))
            (`/Game/ThirdPersonBP/Blueprints/ThirdPersonCharacter.set Health` _player 0.0)))))))

(event `self.Box.OnComponentEndOverlap`
  (params (OverlappedComponent :type "PrimitiveComponent Object Reference") (OtherActor :type "Actor Object Reference") (OtherComp :type "PrimitiveComponent Object Reference") (OtherBodyIndex :type Integer))
  ;[1 1 1] damage over time
  (if (== OtherActor (`self.player`))
    (`KismetSystemLibrary.Delay` 2.0)
    (`TimelineComponent.Stop` (`self.damage over time`))))

(event `self.ReceiveBeginPlay`
  (bind _waypoint_movement (`self.wayPoint Movement`))
  (bind _mygamemanager (`/Game/__MyContent/BluePrints/BP_MyFunctionLibrary.get game manager`))
  (set `self.player` (`/Game/__MyContent/BluePrints/BP_MyGameManager.MyPlayer` _mygamemanager))
  (set `self.times looped` 0)
  (set `self.waypoints` (`|MakeArray` (`self.wayPoint1`) (`self.wayPoint2`) (`self.waypoint 3`)))
  (`TimelineComponent.SetPlayRate` _waypoint_movement (`self.rate`))
  (`self.set first wayPoint`)
  (`TimelineComponent.PlayFromStart` _waypoint_movement))

(fn `path is finished`
  (returns (`path finished` :type Boolean))
  (return (== (`self.nextWaypoint`) (- (`KismetArrayLibrary.Array_Length` (`self.waypoints`)) 1))))

(fn `set first wayPoint`
  (set `self.current waypoint` 0)
  (set `self.nextWaypoint` 1)
  (`self.set positions of waypoints`))

(fn `set next waypoint`
  (bind _result (`/Engine/EditorBlueprintResources/StandardMacros.IncrementInt` (`self.current waypoint`))
    (:`  `
      (set `self.nextWaypoint` (+ _result 1))
      (`self.set positions of waypoints`))))

(fn `set positions of waypoints`
  (bind _waypoints (`self.waypoints`))
  (set `self.current waypoint pos` (`self.K2_GetActorLocation` (`|GetArrayItem` _waypoints (`self.current waypoint`))))
  (set `self.next waypoint position` (`self.K2_GetActorLocation` (`|GetArrayItem` _waypoints (`self.nextWaypoint`)))))

(fn `UserConstructionScript`)