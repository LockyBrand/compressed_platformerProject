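; Waypoint-driven moving platform with configurable mesh and material that can double as an enemy hazard.
; MotionTimeline lerps its location between successive hidden waypoint actors at a set rate, optionally looping from the first when the path finishes.
; When IsEnemy is set, hitting the player activates a burning effect and a DamageOverTime timeline that drains health.
; Start and Stop functions control the motion, while an enemy look-at rotation branch sits unconnected.
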(event `self.ReceiveBeginPlay`
  (for _array_element (`self.waypoints`)
    (`self.SetActorHiddenInGame` _array_element true)
    (`self.platform start`)))

(event `platform start`
  (bind _motion_timeline (`self.motion timeline`))
  (`self.set first waypoint`)
  (`TimelineComponent.SetPlayRate` _motion_timeline (`self.rate`))
  (`TimelineComponent.PlayFromStart` _motion_timeline))

(event `self.platofrm Mesh.OnComponentHit`
  (params (HitComponent :type "PrimitiveComponent Object Reference") (OtherActor :type "Actor Object Reference") (OtherComp :type "PrimitiveComponent Object Reference") (NormalImpulse :type "Vector Structure") (Hit :type "HitResult Structure (by ref)"))
  (bind _mygamemanager (`/Game/__MyContent/BluePrints/BP_MyFunctionLibrary.get game manager`))
  (bind _myplayer (`/Game/__MyContent/BluePrints/BP_MyGameManager.MyPlayer` _mygamemanager))
  (if (== _myplayer OtherActor)
    (if (`self.is enemy?`)
      (`TimelineComponent.PlayFromStart` (`self.damage over time`))
      (`ActorComponent.Activate` (`/Game/ThirdPersonBP/Blueprints/ThirdPersonCharacter.burning` _myplayer) false))))

(fn `path is finished`
  (returns (`path finished` :type Boolean))
  (return (== (`self.next waypoint index`) (- (`KismetArrayLibrary.Array_Length` (`self.waypoints`)) 1))))

(fn `set first waypoint`
  (set `self.current waypoint index` 0)
  (set `self.next waypoint index` 1)
  (`self.set positions`))

(fn `set next waypoint`
  (bind _result (`/Engine/EditorBlueprintResources/StandardMacros.IncrementInt` (`self.current waypoint index`))
    (:`  `
      (set `self.next waypoint index` (+ _result 1))
      (`self.set positions`))))

(fn `set positions`
  (bind _waypoints (`self.waypoints`))
  (set `self.current waypoint position` (`self.K2_GetActorLocation` (`|GetArrayItem` _waypoints (`self.current waypoint index`))))
  (set `self.next way position` (`self.K2_GetActorLocation` (`|GetArrayItem` _waypoints (`self.next waypoint index`)))))

(fn `start`
  (`self.platform start`))

(fn `stop`
  (`TimelineComponent.Stop` (`self.motion timeline`)))

(fn `UserConstructionScript`
  (bind _platofrm_mesh (`self.platofrm Mesh`))
  (`StaticMeshComponent.SetStaticMesh` _platofrm_mesh (`self.static mesh`))
  (`PrimitiveComponent.SetMaterial` _platofrm_mesh 0 (`self.static material`)))