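; BP_mySplinePlatform is a moving platform that starts travelling along a spline when its mesh registers a hit.
; A timeline, played at a configurable rate, maps its normalized distance onto the spline length and sets the mesh's world location without sweeping.
; With Reverse enabled, a toggling Loop flag alternates reverse runs and delayed forward replays.
; The construction script applies the configurable mesh and material.
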(event `self.Platform Mesh.OnComponentHit`
  (params (HitComponent :type "PrimitiveComponent Object Reference") (OtherActor :type "Actor Object Reference") (OtherComp :type "PrimitiveComponent Object Reference") (NormalImpulse :type "Vector Structure") (Hit :type "HitResult Structure (by ref)"))
  (`self.platform start`))

(event `platform start`
  (bind _spline (`self.Spline`))
  (`TimelineComponent.SetPlayRate` (`self.motion timeline`) (`self.rate`))
  (bind (_direction _spline_distance) (`Timeline|motion timeline` :!via `PlayFromStart` :!label _label)
    (:`Update`
      (`SceneComponent.K2_SetWorldLocation` (`self.Platform Mesh`) (`SplineComponent.GetLocationAtDistanceAlongSpline` _spline (* _spline_distance (`SplineComponent.GetSplineLength` _spline)) "World") false false))
    (:`Finished`
      (if (`self.reverse`)
        (if (`self.loop`)
          (set `self.loop` false)
          (`self.reverse_platform`)
          (else
            (set `self.loop` true)
            (`KismetSystemLibrary.Delay` 1.0)
            (`TimelineComponent.PlayFromStart` (`self.motion timeline`))))))))

(event `reverse_platform`
  (goto _label :!via `ReverseFromEnd`))

(fn `UserConstructionScript`
  (`StaticMeshComponent.SetStaticMesh` (`self.Platform Mesh`) (`self.Static Mesh`))
  (`PrimitiveComponent.SetMaterial` (`self.Platform Mesh`) 0 (`self.Material`)))