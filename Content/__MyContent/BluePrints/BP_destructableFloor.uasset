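; A destructible floor Blueprint that can shatter when the player enters its trigger box.
; Overlap by the GameManager's player marks it broken and, if BreakOnPlayer is set, applies radius damage at the destructible component's location.
; The first break plays a sound once, then after a short delay hides the destructible and disables its collision.
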(event `self.Box.OnComponentBeginOverlap`
  (params (OverlappedComponent :type "PrimitiveComponent Object Reference") (OtherActor :type "Actor Object Reference") (OtherComp :type "PrimitiveComponent Object Reference") (OtherBodyIndex :type Integer) (bFromSweep :type Boolean) (SweepResult :type "HitResult Structure (by ref)"))
  (bind _destructible (`self.Destructible`))
  (bind _mygamemanager (`/Game/__MyContent/BluePrints/BP_MyFunctionLibrary.get game manager`))
  (if (== OtherActor (`/Game/__MyContent/BluePrints/BP_MyGameManager.MyPlayer` _mygamemanager))
    (set `self.is broken?` true)
    (if (`self.breakOnPlayer?`)
      (if (`self.is broken?`)
        (`DestructibleComponent.ApplyRadiusDamage` _destructible 20.0 (`SceneComponent.K2_GetComponentLocation` _destructible) 20.0 10.0 false)
        (if (not (`self.has sound played`))
          (`GameplayStatics.PlaySoundAtLocation` "/Game/__MyContent/audio/SC_break.SC_break" (`self.K2_GetActorLocation`) (struct) 1.0 1.0 0.0 null null null)
          (set `self.has sound played` true)
          (`KismetSystemLibrary.Delay` 2.0)
          (`SceneComponent.SetVisibility` (`self.Destructible`) false false)
          (`PrimitiveComponent.SetCollisionEnabled` (`self.Destructible`) "NoCollision"))
        (else
          (`DestructibleComponent.ApplyRadiusDamage` _destructible 0.0 (`SceneComponent.K2_GetComponentLocation` _destructible) 0.0 0.0 false))))))

(fn `UserConstructionScript`)