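; Destructible window wall piece that shatters when the player runs into it.
; On component hit, it checks the other actor against the player held by the GameManager, then applies radius damage at the destructible's own location.
; A break sound plays while IsBroken is false, though this graph never sets that flag.
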(event `self.Destructible.OnComponentHit`
  (params (HitComponent :type "PrimitiveComponent Object Reference") (OtherActor :type "Actor Object Reference") (OtherComp :type "PrimitiveComponent Object Reference") (NormalImpulse :type "Vector Structure") (Hit :type "HitResult Structure (by ref)"))
  (bind _destructible (`self.Destructible`))
  (bind _mygamemanager (`/Game/__MyContent/BluePrints/BP_MyFunctionLibrary.get game manager`))
  (if (== OtherActor (`/Game/__MyContent/BluePrints/BP_MyGameManager.MyPlayer` _mygamemanager))
    (`DestructibleComponent.ApplyRadiusDamage` _destructible 100.0 (`SceneComponent.K2_GetComponentLocation` _destructible) 100.0 0.0 false)
    (if (not (`self.is broken?`))
      (`GameplayStatics.PlaySoundAtLocation` "/Game/__MyContent/audio/SC_break.SC_break" (`self.K2_GetActorLocation`) (struct) 1.0 1.0 0.0 null null null))))

(fn `UserConstructionScript`)